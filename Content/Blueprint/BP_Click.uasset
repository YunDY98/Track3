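; BP_Click is a clickable cube actor that brightens with each click and self-destructs after repeated clicks.
; BeginPlay creates a dynamic material instance, and each of the first five clicks prints the count and raises its Bright parameter.
; From the sixth click, it switches to M_Blink, waits through a delay, calls DestroyActor, then requests an explosion emitter attached to the cube.
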(event OnClicked(Cube)
  (params (TouchedComponent :type Primitive%20Component%20Object%20Reference) (ButtonPressed :type Key%20Structure :default "None"))
  (bind _output_get (Variables|Default|SetNewVar_0 (+ (Variables|Default|GetNewVar_0) 1)))
  (if (> 6 _output_get)
    (Development|PrintString (Utilities|String|ToString(Integer) _output_get))
    (Rendering|Material|SetScalarParameterValue (Variables|Default|GetMat) "Bright" (* _output_get 14.786) :!class /Script/Engine.MaterialInstanceDynamic)
    (else
      (Rendering|Material|SetMaterial (Variables|Default|GetCube) 0 "/Game/Materials/M_Blink.M_Blink")
      (Utilities|FlowControl|Delay 1e+01)
      (Actor|DestroyActor)
      (Effects|SpawnEmitterAttached "/Game/StarterContent/Particles/P_Explosion.P_Explosion" (Variables|Default|GetCube) "None"))))

(event EventBeginPlay
  (bind _returnvalue (Rendering|Material|CreateDynamicMaterialInstance (Variables|Default|GetCube) 0 0 "None" :!class /Script/Engine.PrimitiveComponent))
  (Variables|Default|SetMat _returnvalue))

(event Collision|EventActorBeginOverlap
  (params (OtherActor :type Actor%20Object%20Reference)))

(event EventTick
  (params (DeltaSeconds :type Float%20%28single-precision%29)))

(fn ConstructionScript)